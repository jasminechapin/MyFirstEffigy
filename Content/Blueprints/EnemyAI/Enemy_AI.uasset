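; AI controller for enemies that starts the Enemy_BT behavior tree on BeginPlay and feeds it perception results.
; Perception updates write sensed state to the blackboard: CanSeePlayer for BP_Player, CanSeeOtherEnemy for BP_Enemy.
; For enemies it also stores the actor as VisibleEnemy, on both gaining and losing sight, and ignores other actor types.
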(event OnTargetPerceptionUpdated(AIPerception)
  (params (Actor :type Actor%20Object%20Reference) (Stimulus :type AI%20Stimulus%20Structure))
  (bind _bsuccessfullysensed (Utilities|Struct|BreakAIStimulus Stimulus))
  (bind _returnvalue (AI|GetBlackboard 0))
  (Utilities|Casting|CastToBP_Player Actor
    (:then
      (AI|Components|Blackboard|SetValueasBool (AI|GetBlackboard 0) (Utilities|Name|MakeLiteralName "CanSeePlayer") _bsuccessfullysensed))
    (:CastFailed
      (bind _asbp_enemy (Utilities|Casting|CastToBP_Enemy Actor))
      (AI|Components|Blackboard|SetValueasBool _returnvalue (Utilities|Name|MakeLiteralName "CanSeeOtherEnemy") _bsuccessfullysensed)
      (AI|Components|Blackboard|SetValueasObject _returnvalue (Utilities|Name|MakeLiteralName "VisibleEnemy") _asbp_enemy))))

(event EventBeginPlay
  (AI|RunBehaviorTree "/Game/Blueprints/EnemyAI/Enemy_BT.Enemy_BT"))

(event EventTick
  (params (DeltaSeconds :type Float%20%28single-precision%29)))

(fn ConstructionScript)